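; BP_PCharacter_Primitive is the player character for the Primitives level, handling a simple collect-and-deliver win condition.
; Overlapping an actor tagged WinSphere sets a flag and destroys it.
; Overlapping a WinPlatform-tagged actor while holding the flag shows the UBP_Victory widget, waits briefly, then opens the Primitives level.
; Each tick it draws a short-lived debug point at the capsule's location, leaving a visible movement trail.
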(event Collision|EventActorBeginOverlap
  (params (OtherActor :type Actor%20Object%20Reference))
  (if (Actor|ActorHasTag OtherActor "WinSphere")
    (Variables|Default|SetbHasWinSphere true)
    (Actor|DestroyActor OtherActor)
    (elif (and (Actor|ActorHasTag OtherActor "WinPlatform") (Variables|Default|GetbHasWinSphere))
      (bind _returnvalue (UserInterface|CreateWidget "/Game/Blueprints/UBP_Victory.UBP_Victory_C"))
      (UserInterface|Viewport|AddtoViewport _returnvalue 0)
      (Utilities|FlowControl|Delay 5.0)
      (Game|OpenLevel(byName) "Primitives"))))

(event EventTick
  (params (DeltaSeconds :type Float%20%28single-precision%29))
  (Rendering|Debug|DrawDebugPoint (Transformation|GetWorldLocation (Variables|Default|GetCapsuleComponent)) 5.0 "(R=1.000000,G=0.918643,B=0.972617,A=1.000000)" 1.5))

(fn ConstructionScript)