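; Side-scrolling player character that moves along the X axis, with a fall speed clamp and a coyote-time grace window.
; Tick caps downward velocity at MaxFallingSpeed, also zeroing Y velocity when it does.
; Entering Falling starts a timer, cleared on landing, that the CanJumpInternal override treats as permission to jump.
; Jump input calls LaunchCharacter directly, without consulting that check.
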(event Custom|CoyoteTimePassed
  (Development|PrintString "Timer set"))

(event EventOnMovementModeChanged
  (params (PrevMovementMode :type EMovementMode%20Enum :default "MOVE_None") (NewMovementMode :type EMovementMode%20Enum :default "MOVE_None") (PrevCustomMode :type Byte :default 0) (NewCustomMode :type Byte :default 0))
  (if (Utilities|Enum|Equal(Enum) NewMovementMode "MOVE_Falling")
    (bind _returnvalue (Utilities|Time|SetTimerbyEvent (delegate Custom|CoyoteTimePassed) (Variables|Default|GetCoyoteTime)))
    (Variables|Default|SetCoyoteTimer _returnvalue)))

(event EventOnLanded
  (params (Hit :type Hit%20Result%20Structure%20%28by%20ref%29))
  (Utilities|Time|ClearandInvalidateTimerbyHandle (Variables|Default|GetCoyoteTimer))
  (Development|PrintString "Timer cleared"))

(event EventTick
  (params (DeltaSeconds :type Float%20%28single-precision%29))
  ;[1 1 1] Tick
  (Utilities|FlowControl|Sequence
    (:then_0
      (if (< (.Z (Math|Vector|BreakVector (Variables|/Script/Engine.MovementComponent|GetVelocity (Variables|Character|GetCharacterMovement)))) (Variables|Default|GetMaxFallingSpeed))
        (Variables|/Script/Engine.MovementComponent|SetVelocity (Variables|Character|GetCharacterMovement) (Math|Vector|MakeVector (.X (Math|Vector|BreakVector (Variables|/Script/Engine.MovementComponent|GetVelocity (Variables|Character|GetCharacterMovement)))) 0.0 (Variables|Default|GetMaxFallingSpeed)))))))

(event EventBeginPlay
  ;[1 1 1] Begin PLay
  (Variables|/Script/Engine.CharacterMovementComponent|SetbNotifyApex (Variables|Character|GetCharacterMovement) true))

(event Input|ActionEvents|InputActionJump
  (params (Key :type Key%20Structure :default "None"))
  ;[1 1 1] Input
  (:Pressed
    (Character|LaunchCharacter "0, 0,600.000000" false true)))

(event Input|AxisEvents|InputAxisMoveRight
  (params (AxisValue :type Float%20%28single-precision%29))
  ;[1 1 1] Input
  (Pawn|Input|AddMovementInput "1.000000, 0, 0" AxisValue false))

(fn ConstructionScript)

(fn CanJumpInternal
  (bind _returnvalue (|CallParentFunction))
  (return (or _returnvalue (> (Utilities|Time|GetTimerRemainingTimebyHandle (Variables|Default|GetCoyoteTimer)) 0.0))))