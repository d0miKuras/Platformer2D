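; Paper2D player character with a wizard sprite that dashes horizontally on the Dash input.
; A gameplay-tag state machine component drives it through init and tick delegates, with Idle setting the idle flipbook.
; Dashing launches the character along the X component of the sprite's forward vector, relaunches harder on each state tick, then returns to Idle after a short delay.
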(event InitStateDelegate(m_StateMachine)
  (params (StateTag :type Gameplay%20Tag%20Structure%20%28by%20ref%29))
  (|SwitchGameplayTag StateTag
    (:PlayerState.Idle
      (Sprite|SetFlipbook (Variables|Default|GetSprite) "/Game/Flipbooks/FB_Wizard_Idle.FB_Wizard_Idle"))
    (:PlayerState.Dashing
      (Character|LaunchCharacter (* (Math|Vector|GetForwardVector (Variables|Default|GetSprite)) "1000.000000,0,0") true false)
      (Utilities|FlowControl|Delay 0.5)
      (Class|StateMachineComponent|SwitchState (Variables|Default|Getm_StateMachine) "(TagName=\"PlayerState.Idle\")"))))

(event TickStateDelegate(m_StateMachine)
  (params (DeltaTime :type Float%20%28single-precision%29) (StateTag :type Gameplay%20Tag%20Structure%20%28by%20ref%29))
  (|SwitchGameplayTag StateTag
    (:PlayerState.Dashing
      (Character|LaunchCharacter (* (Math|Vector|GetForwardVector (Variables|Default|GetSprite)) "5000.000000,0,0") true false))))

(event EventBeginPlay)

(event Collision|EventActorBeginOverlap
  (params (OtherActor :type Actor%20Object%20Reference)))

(event EventTick
  (params (DeltaSeconds :type Float%20%28single-precision%29)))

(event Input|ActionEvents|InputActionDash
  (params (Key :type Key%20Structure :default "None"))
  (:Pressed
    (Class|StateMachineComponent|SwitchState (Variables|Default|Getm_StateMachine) "(TagName=\"PlayerState.Dashing\")")))

(fn ConstructionScript)